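; Blueprint function library of casting shortcuts for the Sokoban game's player controller and player pawn.
; GetSokobanPlayercontroller casts player controller 0 to BP_SokobanPlayerController, and GetSokobanPlayer casts that controller's controlled pawn to BP_Player.
; SetMoveInput uses the controller getter to write its AcceptMoveInput flag.
; An additional function, 新函数, is an empty stub.
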(fn `GetSokobanPlayer`
  (returns (SokobanPlayer :type "/Game/Sokoban/Blueprint/Characters/BP_Player Object Reference"))
  (bind _asbp_player (cast `/Game/Sokoban/Blueprint/Characters/BP_Player` (`Controller.K2_GetPawn` (`self.GetSokobanPlayercontroller` null))))
  (return _asbp_player))

(fn `GetSokobanPlayercontroller`
  (returns (`Sokoban Player Controller` :type "/Game/Sokoban/Blueprint/Gameplay/BP_SokobanPlayerController Object Reference"))
  (bind _asbp_sokoban_player_controller (cast `/Game/Sokoban/Blueprint/Gameplay/BP_SokobanPlayerController` (`GameplayStatics.GetPlayerController` null)))
  (return _asbp_sokoban_player_controller))

(fn `SetMoveInput`
  (params (AcceptMoveInput :type Boolean))
  (set `/Game/Sokoban/Blueprint/Gameplay/BP_SokobanPlayerController.AcceptMoveInput` AcceptMoveInput (`self.GetSokobanPlayercontroller` null)))

(fn `新函数`)