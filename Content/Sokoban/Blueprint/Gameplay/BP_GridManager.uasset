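; Sokoban grid manager actor that holds the level's cell layout, converts between grid and world coordinates, and centers a given camera.
; Cell queries report goals, walls and out-of-bounds cells, while box lookups scan all BP_BoxActor instances by their current coordinates.
; BuildGridVisuals rebuilds floors, walls and goals as instanced static meshes, adding box and player stand-ins only in preview mode.
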(event EventBeginPlay)

(event Collision|EventActorBeginOverlap
  (params (OtherActor :type Actor%20Object%20Reference)))

(event EventTick
  (params (DeltaSeconds :type Float%20%28single-precision%29)))

(fn ConstructionScript)

(fn GridtoWorld
  (params (InCoord :type ST%20Grid%20Coord%20Structure))
  (bind (_x _y) (Utilities|Struct|BreakST_GridCoord InCoord))
  (bind _returnvalue (Transformation|GetActorLocation))
  (bind _cellsize (Variables|Default|GetCellSize))
  (return (Math|Vector|MakeVector (+ (* _x _cellsize) (.x _returnvalue)) (+ (* _y _cellsize) (.y _returnvalue)) (.z _returnvalue))))

(fn IsInsideGrid
  (params (InCoord :type ST%20Grid%20Coord%20Structure))
  (bind (_x _y) (Utilities|Struct|BreakST_GridCoord InCoord))
  (return (Math|Boolean|ANDBoolean (>= _x 0) (>= _y 0) (< _x (Variables|Default|GetGridHeight)) (< _y (Variables|Default|GetGridWidth)))))

(fn IsGoal
  (params (InCoord :type ST%20Grid%20Coord%20Structure))
  (return (Utilities|Array|ContainsItem (Variables|Default|GetGoalCells) InCoord)))

(fn IsBox
  (params (InCoord :type ST%20Grid%20Coord%20Structure))
  (bind _box (CallFunction|GetCurrentBox InCoord))
  (return (Utilities|IsValid _box)))

(fn IsWall
  (params (InCoord :type ST%20Grid%20Coord%20Structure))
  (return (Utilities|Array|ContainsItem (Variables|Default|GetWallCells) InCoord)))

(fn CellBlocked
  (params (InCoord :type ST%20Grid%20Coord%20Structure))
  (if (Recognize|IsInsideGrid InCoord)
    (if (Recognize|IsWall InCoord)
      (return true)
      (else
        (return false)))
    (else
      (return true))))

(fn GetCurrentBox
  (params (In%20Coord :type ST%20Grid%20Coord%20Structure))
  (bind (_x _y) (Utilities|Struct|BreakST_GridCoord In%20Coord))
  (bind _outactors (Actor|GetAllActorsOfClass "/Game/Sokoban/Blueprint/Gameplay/BP_BoxActor.BP_BoxActor_C"))
  (for _array_element _outactors
    (if (and (== (Variables|/Game/Sokoban/Blueprint/Gameplay/BP_BoxActor.BP_BoxActor_C|GetCurrentX _array_element) _x) (== (Variables|/Game/Sokoban/Blueprint/Gameplay/BP_BoxActor.BP_BoxActor_C|GetCurrentY _array_element) _y))
      (return _array_element))))

(fn GetAllBoxCoord
  (bind _outactors (Actor|GetAllActorsOfClass "/Game/Sokoban/Blueprint/Gameplay/BP_BoxActor.BP_BoxActor_C"))
  (for _array_element _outactors
    (Utilities|Array|Add (LocalVariables|Get_Boxes) (Utilities|Struct|MakeST_GridCoord (Variables|/Game/Sokoban/Blueprint/Gameplay/BP_BoxActor.BP_BoxActor_C|GetCurrentX _array_element) (Variables|/Game/Sokoban/Blueprint/Gameplay/BP_BoxActor.BP_BoxActor_C|GetCurrentY _array_element))))
  (return (LocalVariables|Get_Boxes)))

(fn BuildGridVisuals
  (params (PreviewMode :type Boolean))
  (bind _cellsize (Variables|Default|GetCellSize))
  (bind _cellsize_2 (Variables|Default|GetCellSize))
  (bind _cellsize_3 (Variables|Default|GetCellSize))
  (bind _cellsize_4 (Variables|Default|GetCellSize))
  (bind _cellsize_5 (Variables|Default|GetCellSize))
  (bind _returnvalue (/ _cellsize_3 1e+02))
  (bind _returnvalue_2 (/ _cellsize_2 1e+02))
  (bind _returnvalue_3 (/ _cellsize_4 1e+02))
  (bind _returnvalue_4 (/ _cellsize_5 1e+02))
  (bind _returnvalue_5 (/ _cellsize 2e+02))
  (bind _returnvalue_6 (* _returnvalue_2 0.9))
  (bind _returnvalue_7 (* _returnvalue 0.9))
  (Utilities|FlowControl|Sequence
    (:then_0
      (Components|InstancedStaticMesh|ClearInstances (Variables|Default|GetISM_Walls))
      (Components|InstancedStaticMesh|ClearInstances (Variables|Default|GetISM_Floor))
      (Components|InstancedStaticMesh|ClearInstances (Variables|Default|GetISM_Goals))
      (Components|InstancedStaticMesh|ClearInstances (Variables|Default|GetISM_BoxesPreview))
      (Components|InstancedStaticMesh|ClearInstances (Variables|Default|GetISM_PlayerPreview))
      (Components|InstancedStaticMesh|ClearInstances (Variables|Default|GetISM_Guide)))
    (:then_2
      ;[0.15 0.15 0.15 0.5] Spawn Walls
      (for _array_element (Variables|Default|GetWallCells)
        (bind _worldlocation (Transform|GridtoWorld _array_element))
        (Components|InstancedStaticMesh|AddInstance (Variables|Default|GetISM_Walls) (Math|Transform|MakeTransform (Math|Vector|MakeVector (.x _worldlocation) (.y _worldlocation) (+ (.z _worldlocation) 1e+02)) "0, 0, 0" (Math|Vector|MakeVector _returnvalue_4 _returnvalue_4 _returnvalue_4)) false)
        (CallFunction|AddFloorInstrnce (Math|Vector|MakeVector (.x _worldlocation) (.y _worldlocation) (.z _worldlocation)))))
    (:then_3
      ;[0.15 0.15 0.15 0.5] Spawn Goals
      (for _array_element_2 (Variables|Default|GetGoalCells)
        (bind _worldlocation_2 (Transform|GridtoWorld _array_element_2))
        (Components|InstancedStaticMesh|AddInstance (Variables|Default|GetISM_Goals) (Math|Transform|MakeTransform (Math|Vector|MakeVector (.x _worldlocation_2) (.y _worldlocation_2) (+ (.z _worldlocation_2) 5.0)) "0, 0, 0" (Math|Vector|MakeVector _returnvalue_6 _returnvalue_6 0.1)) false)
        (CallFunction|AddFloorInstrnce (Math|Vector|MakeVector (.x _worldlocation_2) (.y _worldlocation_2) (.z _worldlocation_2)))))
    (:then_4
      (for _array_element_3 (Variables|Default|GetFloorCells)
        (bind _worldlocation_3 (Transform|GridtoWorld _array_element_3))
        (Components|InstancedStaticMesh|AddInstance (Variables|Default|GetISM_Floor) (Math|Transform|MakeTransform (Math|Vector|MakeVector (.x _worldlocation_3) (.y _worldlocation_3) (+ (.z _worldlocation_3) 5.0)) "0, 0, 0" (Math|Vector|MakeVector _returnvalue_3 _returnvalue_3 0.1)) false)))
    (:then_5
      ;[0.15 0.15 0.15 0.5] Preview Item
      (for _array_element_4 (Variables|Default|GetBoxCells)
        (bind _worldlocation_4 (Transform|GridtoWorld _array_element_4))
        (CallFunction|AddFloorInstrnce (Math|Vector|MakeVector (.x _worldlocation_4) (.y _worldlocation_4) (.z _worldlocation_4)))
        (if PreviewMode
          (Components|InstancedStaticMesh|AddInstance (Variables|Default|GetISM_BoxesPreview) (Math|Transform|MakeTransform (Math|Vector|MakeVector (.x _worldlocation_4) (.y _worldlocation_4) (+ (.z _worldlocation_4) 9e+01)) "0, 0, 0" (Math|Vector|MakeVector _returnvalue_7 _returnvalue_7 _returnvalue_7)) false))))
    (:then_6
      (bind _worldlocation_5 (Transform|GridtoWorld (Variables|Default|GetPlayerPreview)))
      (CallFunction|AddFloorInstrnce (Math|Vector|MakeVector (.x _worldlocation_5) (.y _worldlocation_5) (.z _worldlocation_5)))
      (if PreviewMode
        (Components|InstancedStaticMesh|AddInstance (Variables|Default|GetISM_PlayerPreview) (Math|Transform|MakeTransform (Math|Vector|MakeVector (.x _worldlocation_5) (.y _worldlocation_5) (+ (.z _worldlocation_5) 1e+02)) "0, 0, 0" (Math|Vector|MakeVector _returnvalue_5 _returnvalue_5 (/ (Variables|Default|GetCellSize) 1e+02))) false)))))

(fn WorldtoGrid
  (params (WorldLocation :type Vector))
  (bind _returnvalue (Transformation|GetActorLocation))
  (return (Utilities|Struct|MakeST_GridCoord (Math|Float|Floor (/ (- (.x WorldLocation) (.x _returnvalue)) (Variables|Default|GetCellSize))) (Math|Float|Floor (/ (- (.y WorldLocation) (.y _returnvalue)) (Variables|Default|GetCellSize))))))

(fn CenterCamera
  (params (TargetCamera :type Camera%20Actor%20Object%20Reference))
  (Transformation|SetActorLocation TargetCamera (Math|Vector|MakeVector (- (|(((X-1)/2)*Size) (Math|Conversions|ToFloat(Integer) (Variables|Default|GetGridHeight)) (Variables|Default|GetCellSize)) (* (Variables|Default|GetCellSize) 2.5)) (|(((X-1)/2)*Size) (Math|Conversions|ToFloat(Integer) (Variables|Default|GetGridWidth)) (Variables|Default|GetCellSize)) 1.55e+03) false false))

(fn AddFloorInstrnce
  (params (Location :type Vector))
  (bind _cellsize (Variables|Default|GetCellSize))
  (bind _returnvalue (/ _cellsize 1e+02))
  (Components|InstancedStaticMesh|AddInstance (Variables|Default|GetISM_Floor) (Math|Transform|MakeTransform Location "0, 0, 0" (Math|Vector|MakeVector _returnvalue _returnvalue 0.1)) false))