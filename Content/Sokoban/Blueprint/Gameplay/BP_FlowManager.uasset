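; BP_FlowManager drives the Sokoban game flow between main menu, level select and gameplay.
; It tracks flow state, selected level and highest unlocked level, raising the unlock when a level is completed.
; Transitions disable input and blend between menu and gameplay cameras, with timers matched to the blend time.
; Finish functions swap menu and HUD and restore input; returning also reloads the selected level through BP_LevelManager.
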(event `self.ReceiveBeginPlay`
  (set `self.PlayerControllerRef` (`/Game/Sokoban/Blueprint/BPFL/BPFL_Cast.GetSokobanPlayercontroller`))
  (bind _returnvalue (`GameplayStatics.GetActorOfClass` "/Game/Sokoban/Blueprint/Gameplay/BP_LevelManager.BP_LevelManager_C"))
  (set `self.LevelManagerRef` _returnvalue)
  (`self.Init`))

(fn `BeginTransitionToGameplay`
  (params (LevelIndex :type Integer))
  (set `self.CurrentState` "NewEnumerator2")
  (`/Game/Sokoban/Blueprint/Gameplay/BP_SokobanController.DisableAllInputMappings` (`self.PlayerControllerRef`))
  (set `Widget.Visibility` "Hidden" (`self.MenuRef`))
  (`PlayerController.SetViewTargetWithBlend` (`self.PlayerControllerRef`) (`self.GameplayCameraRef`) (`self.TransitionBlendTime`) "VTBlend_Linear" 0.0 false)
  (`KismetSystemLibrary.K2_SetTimerDelegate` (`|CreateDelegate` :!event `FinishTransitionToGameplay`) (`self.TransitionBlendTime`)))

(fn `FinishReturnToLevelSelect`
  (bind _menuref (`self.MenuRef`))
  (`Widget.RemoveFromParent` (`self.HUDRef`))
  (`Widget.SetVisibility` _menuref "Visible")
  (`/Game/Sokoban/Blueprint/UI/WBP_MainMenu.OpenLevelSelectPage` _menuref)
  (`/Game/Sokoban/Blueprint/Gameplay/BP_LevelManager.LoadLevelByIndex` (`self.LevelManagerRef`) (`self.SelectedLevelIndex`))
  (`/Game/Sokoban/Blueprint/Gameplay/BP_SokobanController.SwitchToMenuInput` (`self.PlayerControllerRef`))
  (set `self.CurrentState` "NewEnumerator1"))

(fn `FinishTransitionToGameplay`
  (bind _returnvalue (`|CreateWidget` "/Game/Sokoban/Blueprint/UI/WBP_HUD.WBP_HUD_C"))
  (`UserWidget.AddToViewport` _returnvalue 0)
  (set `self.HUDRef` _returnvalue)
  (`/Game/Sokoban/Blueprint/Gameplay/BP_SokobanController.SwitchToGameplayInput` (`self.PlayerControllerRef`))
  (set `self.CurrentState` "NewEnumerator3"))

(fn `Init`
  (bind _menuref (`self.MenuRef`))
  (set `self.CurrentState` "NewEnumerator0")
  (set `self.SelectedLevelIndex` 0)
  (set `self.HighestUnlockedLevelIndex` 1)
  (bind _returnvalue (`|CreateWidget` "/Game/Sokoban/Blueprint/UI/WBP_MainMenu.WBP_MainMenu_C"))
  (bind _output_get (set `self.MenuRef` _returnvalue))
  (`UserWidget.AddToViewport` _output_get 0)
  (`/Game/Sokoban/Blueprint/UI/WBP_MainMenu.InitWithFlowManager` _menuref self)
  (`/Game/Sokoban/Blueprint/UI/WBP_MainMenu.OpenMainPage` _menuref)
  (`/Game/Sokoban/Blueprint/Gameplay/BP_SokobanController.SwitchToMenuInput` (`self.PlayerControllerRef`))
  (`PlayerController.SetViewTargetWithBlend` (`self.PlayerControllerRef`) (`self.MenuCameraRef`) 0.0 "VTBlend_Linear" 0.0 false))

(fn `ReturnToLevelSelectAfterSuccess`
  (params (CompletedLevelIndex :type Integer))
  (set `self.CurrentState` "NewEnumerator4")
  (`/Game/Sokoban/Blueprint/Gameplay/BP_SokobanController.DisableAllInputMappings` (`self.PlayerControllerRef`))
  (set `self.HighestUnlockedLevelIndex` (`KismetMathLibrary.Max` (`self.HighestUnlockedLevelIndex`) (+ (`local.CompletedLevelIndex`) 1)))
  (set `self.SelectedLevelIndex` (`local.CompletedLevelIndex`))
  (`PlayerController.SetViewTargetWithBlend` (`self.PlayerControllerRef`) (`self.MenuCameraRef`) (`self.TransitionBlendTime`) "VTBlend_Linear" 0.0 false)
  (`KismetSystemLibrary.K2_SetTimerDelegate` (`|CreateDelegate` :!event `FinishReturnToLevelSelect`) (`self.TransitionBlendTime`)))

(fn `ReturnToLevelSelectManually`
  (set `self.CurrentState` "NewEnumerator4")
  (`/Game/Sokoban/Blueprint/Gameplay/BP_SokobanController.DisableAllInputMappings` (`self.PlayerControllerRef`))
  (`PlayerController.SetViewTargetWithBlend` (`self.PlayerControllerRef`) (`self.MenuCameraRef`) (`self.TransitionBlendTime`) "VTBlend_Linear" 0.0 false)
  (`KismetSystemLibrary.K2_SetTimerDelegate` (`|CreateDelegate` :!event `FinishReturnToLevelSelect`) (`self.TransitionBlendTime`)))

(fn `UserConstructionScript`)