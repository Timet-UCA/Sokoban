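; Player controller for the Sokoban game that turns Enhanced Input actions into menu navigation and puzzle commands.
; On BeginPlay it caches the level manager, flow manager and player, then forwards grid moves to the player, restart, undo and next level to the level manager, and menu actions to FlowManager's menu.
; Helper functions swap or clear menu and gameplay mapping contexts.
; Back-to-menu quits if TestLevelManager is set, otherwise returns to level select.
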(event `self.ReceiveBeginPlay`
  (bind _returnvalue (`GameplayStatics.GetActorOfClass` "/Game/Sokoban/Blueprint/Gameplay/BP_LevelManager.BP_LevelManager_C"))
  (set `self.LevelManagerRef` _returnvalue)
  (bind _returnvalue_2 (`GameplayStatics.GetActorOfClass` "/Game/Sokoban/Blueprint/Gameplay/BP_FlowManager.BP_FlowManager_C"))
  (set `self.FlowManagerRef` _returnvalue_2)
  (set `self.PlayerRef` (`/Game/Sokoban/Blueprint/BPFL/BPFL_Cast.GetSokobanPlayer`)))

(event `EnhancedInput|/Game/Sokoban/Input/IA_Menu/IA_MenuUp`
  (params (ActionValue :type Boolean) (ElapsedSeconds :type "Float (double-precision)") (TriggeredSeconds :type "Float (double-precision)") (InputAction :type "InputAction Object Reference" :default "/Game/Sokoban/Input/IA_Menu/IA_MenuUp.IA_MenuUp"))
  ; Menu Input
  (:`Triggered`
    (`/Game/Sokoban/Blueprint/UI/WBP_MainMenu.MoveVertical` (`/Game/Sokoban/Blueprint/Gameplay/BP_FlowManager.MenuRef` (`self.FlowManagerRef`)) -1)))

(event `EnhancedInput|/Game/Sokoban/Input/IA_Gameplay/IA_MoveLeft`
  (params (ActionValue :type Boolean) (ElapsedSeconds :type "Float (double-precision)") (TriggeredSeconds :type "Float (double-precision)") (InputAction :type "InputAction Object Reference" :default "/Game/Sokoban/Input/IA_Gameplay/IA_MoveLeft.IA_MoveLeft"))
  ; Gameplay Input
  ;; (A)左-Y
  (:`Triggered`
    (`/Game/Sokoban/Blueprint/Characters/BP_Player.TryMove` (`self.PlayerRef`) 0 -1)))

(event `EnhancedInput|/Game/Sokoban/Input/IA_Gameplay/IA_MoveUp`
  (params (ActionValue :type Boolean) (ElapsedSeconds :type "Float (double-precision)") (TriggeredSeconds :type "Float (double-precision)") (InputAction :type "InputAction Object Reference" :default "/Game/Sokoban/Input/IA_Gameplay/IA_MoveUp.IA_MoveUp"))
  ; Gameplay Input
  ;; (W)上+X
  (:`Triggered`
    (`/Game/Sokoban/Blueprint/Characters/BP_Player.TryMove` (`self.PlayerRef`) 1 0)))

(event `EnhancedInput|/Game/Sokoban/Input/IA_Menu/IA_MenuDown`
  (params (ActionValue :type Boolean) (ElapsedSeconds :type "Float (double-precision)") (TriggeredSeconds :type "Float (double-precision)") (InputAction :type "InputAction Object Reference" :default "/Game/Sokoban/Input/IA_Menu/IA_MenuDown.IA_MenuDown"))
  ; Menu Input
  (:`Triggered`
    (`/Game/Sokoban/Blueprint/UI/WBP_MainMenu.MoveVertical` (`/Game/Sokoban/Blueprint/Gameplay/BP_FlowManager.MenuRef` (`self.FlowManagerRef`)) 1)))

(event `EnhancedInput|/Game/Sokoban/Input/IA_Gameplay/IA_MoveRight`
  (params (ActionValue :type Boolean) (ElapsedSeconds :type "Float (double-precision)") (TriggeredSeconds :type "Float (double-precision)") (InputAction :type "InputAction Object Reference" :default "/Game/Sokoban/Input/IA_Gameplay/IA_MoveRight.IA_MoveRight"))
  ; Gameplay Input
  ;; (D)右+Y
  (:`Triggered`
    (`/Game/Sokoban/Blueprint/Characters/BP_Player.TryMove` (`self.PlayerRef`) 0 1)))

(event `EnhancedInput|/Game/Sokoban/Input/IA_Gameplay/IA_MoveDown`
  (params (ActionValue :type Boolean) (ElapsedSeconds :type "Float (double-precision)") (TriggeredSeconds :type "Float (double-precision)") (InputAction :type "InputAction Object Reference" :default "/Game/Sokoban/Input/IA_Gameplay/IA_MoveDown.IA_MoveDown"))
  ; Gameplay Input
  ;; (S)下-X
  (:`Triggered`
    (`/Game/Sokoban/Blueprint/Characters/BP_Player.TryMove` (`self.PlayerRef`) -1 0)))

(event `EnhancedInput|/Game/Sokoban/Input/IA_Menu/IA_MenuLeft`
  (params (ActionValue :type Boolean) (ElapsedSeconds :type "Float (double-precision)") (TriggeredSeconds :type "Float (double-precision)") (InputAction :type "InputAction Object Reference" :default "/Game/Sokoban/Input/IA_Menu/IA_MenuLeft.IA_MenuLeft"))
  ; Menu Input
  (:`Triggered`
    (`/Game/Sokoban/Blueprint/UI/WBP_MainMenu.MoveHorizontal` (`/Game/Sokoban/Blueprint/Gameplay/BP_FlowManager.MenuRef` (`self.FlowManagerRef`)) -1)))

(event `EnhancedInput|/Game/Sokoban/Input/IA_Menu/IA_MenuRight`
  (params (ActionValue :type Boolean) (ElapsedSeconds :type "Float (double-precision)") (TriggeredSeconds :type "Float (double-precision)") (InputAction :type "InputAction Object Reference" :default "/Game/Sokoban/Input/IA_Menu/IA_MenuRight.IA_MenuRight"))
  ; Menu Input
  (:`Triggered`
    (`/Game/Sokoban/Blueprint/UI/WBP_MainMenu.MoveHorizontal` (`/Game/Sokoban/Blueprint/Gameplay/BP_FlowManager.MenuRef` (`self.FlowManagerRef`)) 1)))

(event `EnhancedInput|/Game/Sokoban/Input/IA_Gameplay/IA_Restart`
  (params (ActionValue :type Boolean) (ElapsedSeconds :type "Float (double-precision)") (TriggeredSeconds :type "Float (double-precision)") (InputAction :type "InputAction Object Reference" :default "/Game/Sokoban/Input/IA_Gameplay/IA_Restart.IA_Restart"))
  (bind _levelmanagerref (`self.LevelManagerRef`))
  ; Gameplay Input
  ;; (R)重开
  (:`Triggered`
    (`/Engine/EditorBlueprintResources/StandardMacros.IsValid` _levelmanagerref
      (:`Is Valid`
        (`/Game/Sokoban/Blueprint/Gameplay/BP_LevelManager.RestartCurrentLevel` _levelmanagerref)))))

(event `EnhancedInput|/Game/Sokoban/Input/IA_Menu/IA_MenuConfirm`
  (params (ActionValue :type Boolean) (ElapsedSeconds :type "Float (double-precision)") (TriggeredSeconds :type "Float (double-precision)") (InputAction :type "InputAction Object Reference" :default "/Game/Sokoban/Input/IA_Menu/IA_MenuConfirm.IA_MenuConfirm"))
  ; Menu Input
  (:`Triggered`
    (`/Game/Sokoban/Blueprint/UI/WBP_MainMenu.ConfirmSelection` (`/Game/Sokoban/Blueprint/Gameplay/BP_FlowManager.MenuRef` (`self.FlowManagerRef`)))))

(event `EnhancedInput|/Game/Sokoban/Input/IA_Gameplay/IA_Undo`
  (params (ActionValue :type Boolean) (ElapsedSeconds :type "Float (double-precision)") (TriggeredSeconds :type "Float (double-precision)") (InputAction :type "InputAction Object Reference" :default "/Game/Sokoban/Input/IA_Gameplay/IA_Undo.IA_Undo"))
  (bind _levelmanagerref (`self.LevelManagerRef`))
  ; Gameplay Input
  ;; (Z) Undo
  (:`Triggered`
    (`/Engine/EditorBlueprintResources/StandardMacros.IsValid` _levelmanagerref
      (:`Is Valid`
        (`/Game/Sokoban/Blueprint/Gameplay/BP_LevelManager.UndoLastStep` _levelmanagerref)))))

(event `EnhancedInput|/Game/Sokoban/Input/IA_Menu/IA_MenuBack`
  (params (ActionValue :type Boolean) (ElapsedSeconds :type "Float (double-precision)") (TriggeredSeconds :type "Float (double-precision)") (InputAction :type "InputAction Object Reference" :default "/Game/Sokoban/Input/IA_Menu/IA_MenuBack.IA_MenuBack"))
  ; Menu Input
  (:`Triggered`
    (`/Game/Sokoban/Blueprint/UI/WBP_MainMenu.BackAction` (`/Game/Sokoban/Blueprint/Gameplay/BP_FlowManager.MenuRef` (`self.FlowManagerRef`)))))

(event `EnhancedInput|/Game/Sokoban/Input/IA_Menu/IA_BackToMenu`
  (params (ActionValue :type Boolean) (ElapsedSeconds :type "Float (double-precision)") (TriggeredSeconds :type "Float (double-precision)") (InputAction :type "InputAction Object Reference" :default "/Game/Sokoban/Input/IA_Menu/IA_BackToMenu.IA_BackToMenu"))
  ; Gameplay Input
  ;; (ESC)Main Menu
  (:`Triggered`
    (if (`/Game/Sokoban/Blueprint/Gameplay/BP_LevelManager.TestLevelManager` (`self.LevelManagerRef`))
      (`KismetSystemLibrary.QuitGame` null "Quit")
      (else
        (`/Game/Sokoban/Blueprint/Gameplay/BP_FlowManager.ReturnToLevelSelectManually` (`self.FlowManagerRef`))))))

(event `EnhancedInput|/Game/Sokoban/Input/IA_Gameplay/IA_NextLevel`
  (params (ActionValue :type Boolean) (ElapsedSeconds :type "Float (double-precision)") (TriggeredSeconds :type "Float (double-precision)") (InputAction :type "InputAction Object Reference" :default "/Game/Sokoban/Input/IA_Gameplay/IA_NextLevel.IA_NextLevel"))
  (bind _levelmanagerref (`self.LevelManagerRef`))
  (:`Triggered`
    (`/Engine/EditorBlueprintResources/StandardMacros.IsValid` _levelmanagerref
      (:`Is Valid`
        (`/Game/Sokoban/Blueprint/Gameplay/BP_LevelManager.LoadNextLevel` _levelmanagerref)))))

(fn `DisableAllInputMappings`
  (`EnhancedInputSubsystemInterface.ClearAllMappings` (pcsubsystem `EnhancedInputLocalPlayerSubsystem` (`/Game/Sokoban/Blueprint/BPFL/BPFL_Cast.GetSokobanPlayercontroller`))))

(fn `SwitchToGameplayInput`
  (bind _returnvalue (pcsubsystem `EnhancedInputLocalPlayerSubsystem` (`/Game/Sokoban/Blueprint/BPFL/BPFL_Cast.GetSokobanPlayercontroller`)))
  (`EnhancedInputSubsystemInterface.ClearAllMappings` _returnvalue)
  (`EnhancedInputSubsystemInterface.AddMappingContext` _returnvalue "/Game/Sokoban/Input/IMC_Gameplay.IMC_Gameplay" 0 (struct)))

(fn `SwitchToMenuInput`
  (bind _returnvalue (pcsubsystem `EnhancedInputLocalPlayerSubsystem` (`/Game/Sokoban/Blueprint/BPFL/BPFL_Cast.GetSokobanPlayercontroller`)))
  (`EnhancedInputSubsystemInterface.ClearAllMappings` _returnvalue)
  (`EnhancedInputSubsystemInterface.AddMappingContext` _returnvalue "/Game/Sokoban/Input/IMC_Menu.IMC_Menu" 0 (struct)))

(fn `UserConstructionScript`)