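; Player controller for the Sokoban game that maps Enhanced Input actions to grid movement and level commands.
; On BeginPlay it adds the gameplay mapping context and caches the level manager and player pawn.
; Directional inputs call TryMove on the pawn with unit grid steps, gated by AcceptMoveInput.
; Restart, undo and next-level inputs forward to the level manager, while back-to-menu opens the main menu level.
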(event `self.ReceiveBeginPlay`
  (`EnhancedInputSubsystemInterface.AddMappingContext` (pcsubsystem `EnhancedInputLocalPlayerSubsystem` (`GameplayStatics.GetPlayerController` 0)) "/Game/Sokoban/Input/IMC_Gameplay.IMC_Gameplay" 0 (struct))
  (bind _returnvalue (`GameplayStatics.GetActorOfClass` "/Game/Sokoban/Blueprint/Gameplay/BP_LevelManager.BP_LevelManager_C"))
  (set `self.LevelManagerRef` _returnvalue)
  (set `self.ControlledPawnRef` (`/Game/Sokoban/Blueprint/BPFL/BPFL_Cast.GetSokobanPlayer`)))

(event `EnhancedInput|/Game/Sokoban/Input/IA/IA_MoveUp`
  (params (ActionValue :type Boolean) (ElapsedSeconds :type "Float (double-precision)") (TriggeredSeconds :type "Float (double-precision)") (InputAction :type "InputAction Object Reference" :default "/Game/Sokoban/Input/IA/IA_MoveUp.IA_MoveUp"))
  ; (W)上+X
  (:`Triggered`
    (if (`self.AcceptMoveInput`)
      (`/Game/Sokoban/Blueprint/Characters/BP_Player.TryMove` (`self.ControlledPawnRef`) 1 0))))

(event `EnhancedInput|/Game/Sokoban/Input/IA/IA_MoveLeft`
  (params (ActionValue :type Boolean) (ElapsedSeconds :type "Float (double-precision)") (TriggeredSeconds :type "Float (double-precision)") (InputAction :type "InputAction Object Reference" :default "/Game/Sokoban/Input/IA/IA_MoveLeft.IA_MoveLeft"))
  ; (A)左-Y
  (:`Triggered`
    (if (`self.AcceptMoveInput`)
      (`/Game/Sokoban/Blueprint/Characters/BP_Player.TryMove` (`self.ControlledPawnRef`) 0 -1))))

(event `EnhancedInput|/Game/Sokoban/Input/IA/IA_MoveDown`
  (params (ActionValue :type Boolean) (ElapsedSeconds :type "Float (double-precision)") (TriggeredSeconds :type "Float (double-precision)") (InputAction :type "InputAction Object Reference" :default "/Game/Sokoban/Input/IA/IA_MoveDown.IA_MoveDown"))
  ; (S)下-X
  (:`Triggered`
    (if (`self.AcceptMoveInput`)
      (`/Game/Sokoban/Blueprint/Characters/BP_Player.TryMove` (`self.ControlledPawnRef`) -1 0))))

(event `EnhancedInput|/Game/Sokoban/Input/IA/IA_MoveRight`
  (params (ActionValue :type Boolean) (ElapsedSeconds :type "Float (double-precision)") (TriggeredSeconds :type "Float (double-precision)") (InputAction :type "InputAction Object Reference" :default "/Game/Sokoban/Input/IA/IA_MoveRight.IA_MoveRight"))
  ; (D)右+Y
  (:`Triggered`
    (if (`self.AcceptMoveInput`)
      (`/Game/Sokoban/Blueprint/Characters/BP_Player.TryMove` (`self.ControlledPawnRef`) 0 1))))

(event `EnhancedInput|/Game/Sokoban/Input/IA/IA_Restart`
  (params (ActionValue :type Boolean) (ElapsedSeconds :type "Float (double-precision)") (TriggeredSeconds :type "Float (double-precision)") (InputAction :type "InputAction Object Reference" :default "/Game/Sokoban/Input/IA/IA_Restart.IA_Restart"))
  (bind _levelmanagerref (`self.LevelManagerRef`))
  ; (R)重开
  (:`Triggered`
    (`/Engine/EditorBlueprintResources/StandardMacros.IsValid` _levelmanagerref
      (:`Is Valid`
        (`/Game/Sokoban/Blueprint/Gameplay/BP_LevelManager.RestartCurrentLevel` _levelmanagerref)))))

(event `EnhancedInput|/Game/Sokoban/Input/IA/IA_BackToMenu`
  (params (ActionValue :type Boolean) (ElapsedSeconds :type "Float (double-precision)") (TriggeredSeconds :type "Float (double-precision)") (InputAction :type "InputAction Object Reference" :default "/Game/Sokoban/Input/IA/IA_BackToMenu.IA_BackToMenu"))
  ; (ESC)Main Menu
  (:`Triggered`
    (`GameplayStatics.OpenLevel` "Lv_Main")))

(event `EnhancedInput|/Game/Sokoban/Input/IA/IA_Undo`
  (params (ActionValue :type Boolean) (ElapsedSeconds :type "Float (double-precision)") (TriggeredSeconds :type "Float (double-precision)") (InputAction :type "InputAction Object Reference" :default "/Game/Sokoban/Input/IA/IA_Undo.IA_Undo"))
  (bind _levelmanagerref (`self.LevelManagerRef`))
  ; (R) Undo
  (:`Triggered`
    (`/Engine/EditorBlueprintResources/StandardMacros.IsValid` _levelmanagerref
      (:`Is Valid`
        (`/Game/Sokoban/Blueprint/Gameplay/BP_LevelManager.UndoLastStep` _levelmanagerref)))))

(event `EnhancedInput|/Game/Sokoban/Input/IA/IA_NextLevel`
  (params (ActionValue :type Boolean) (ElapsedSeconds :type "Float (double-precision)") (TriggeredSeconds :type "Float (double-precision)") (InputAction :type "InputAction Object Reference" :default "/Game/Sokoban/Input/IA/IA_NextLevel.IA_NextLevel"))
  (bind _levelmanagerref (`self.LevelManagerRef`))
  (:`Triggered`
    (`/Engine/EditorBlueprintResources/StandardMacros.IsValid` _levelmanagerref
      (:`Is Valid`
        (`/Game/Sokoban/Blueprint/Gameplay/BP_LevelManager.LoadNextLevel` _levelmanagerref)))))

(fn `UserConstructionScript`)