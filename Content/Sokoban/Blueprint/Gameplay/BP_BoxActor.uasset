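; BP_BoxActor is a Sokoban box that sits on a grid cell and tracks whether it is on a goal.
; On BeginPlay it finds the BP_GridManager, snaps to its stored cell with a height offset, and checks goal state.
; MoveToCell updates the coordinates, then repeats the snap and check.
; The goal check swaps the mesh material on a goal cell but never restores it off one.
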(event `self.ReceiveBeginPlay`
  (`self.Init`))

(event `self.ReceiveTick`
  (params (DeltaSeconds :type "Float (single-precision)")))

(fn `Init`
  (bind _returnvalue (`GameplayStatics.GetActorOfClass` "/Game/Sokoban/Blueprint/Gameplay/BP_GridManager.BP_GridManager_C"))
  (set `self.GridManagerRef` _returnvalue)
  (`self.SnapToCurrentGrid`)
  (`self.RefreshGoalState`))

(fn `MoveToCell`
  (params (NewX :type Integer) (NewY :type Integer))
  (set `self.CurrentX` NewX)
  (set `self.CurrentY` NewY)
  (`self.SnapToCurrentGrid`)
  (`self.RefreshGoalState`))

(fn `RefreshGoalState`
  (`/Engine/EditorBlueprintResources/StandardMacros.IsValid` (`self.GridManagerRef`)
    (:`Is Valid`
      (bind _output_get (set `self.OnGoal` (`/Game/Sokoban/Blueprint/Gameplay/BP_GridManager.IsGoal` (`self.GridManagerRef`) (make `/Game/Sokoban/Blueprint/Structure/ST_GridCoord` (`self.CurrentX`) (`self.CurrentY`)))))
      (if _output_get
        (`PrimitiveComponent.SetMaterial` (`self.StaticMesh`) 0 "/Engine/MapTemplates/Materials/BasicAsset01.BasicAsset01")))))

(fn `SnapToCurrentGrid`
  (`/Engine/EditorBlueprintResources/StandardMacros.IsValid` (`self.GridManagerRef`)
    (:`Is Valid`
      (bind _worldlocation (`/Game/Sokoban/Blueprint/Gameplay/BP_GridManager.GridToWorld` (`self.GridManagerRef`) (make `/Game/Sokoban/Blueprint/Structure/ST_GridCoord` (`self.CurrentX`) (`self.CurrentY`))))
      (`self.K2_SetActorLocation` (`KismetMathLibrary.MakeVector` (.x _worldlocation) (.y _worldlocation) (+ (.z _worldlocation) (`self.BoxZOffset`)))))))

(fn `UserConstructionScript`)