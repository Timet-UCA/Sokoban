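; Level manager for a Sokoban game that loads levels from the LevelDB save slot and handles restart, next level and undo.
; Loading a level pushes its cells into the grid manager, snaps the player, spawns boxes and centers the camera.
; Undo keeps a capped stack of player and box coordinate snapshots.
; Success returns to level select through the flow manager, while a test flag enables standalone play with its own camera and HUD.
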(event `self.ReceiveBeginPlay`
  (bind _sokoban_player_controller (`/Game/Sokoban/Blueprint/BPFL/BPFL_Cast.GetSokobanPlayercontroller`))
  (bind _returnvalue (`GameplayStatics.GetActorOfClass` "/Game/Sokoban/Blueprint/Gameplay/BP_GridManager.BP_GridManager_C"))
  (set `self.GridManagerRef` _returnvalue)
  (bind _returnvalue_2 (`GameplayStatics.GetActorOfClass` "/Game/Sokoban/Blueprint/Characters/BP_Player.BP_Player_C"))
  (set `self.PlayerRef` _returnvalue_2)
  (bind _returnvalue_3 (`GameplayStatics.GetActorOfClass` "/Game/Sokoban/Blueprint/Gameplay/BP_FlowManager.BP_FlowManager_C"))
  (set `self.FlowManagerRef` _returnvalue_3)
  ; 读取存档
  (bind _returnvalue_4 (`GameplayStatics.DoesSaveGameExist` "LevelDB"))
  (if _returnvalue_4
    (bind _returnvalue_5 (`GameplayStatics.LoadGameFromSlot` "LevelDB"))
    (set `self.LevelDatabaseRef` (cast `/Game/Sokoban/Blueprint/Data/SG_LevelDatabase` _returnvalue_5 :!pure true))
    (else
      (bind _returnvalue_6 (`GameplayStatics.CreateSaveGameObject` "/Game/Sokoban/Blueprint/Data/SG_LevelDatabase.SG_LevelDatabase_C"))
      (set `self.LevelDatabaseRef` _returnvalue_6)))
  (set `self.LevelList` (`/Game/Sokoban/Blueprint/Data/SG_LevelDatabase.SavedLevels` (`self.LevelDatabaseRef`)))
  (if (`self.TestLevelManager`)
    (`self.LoadLevelByIndex` (`self.TestLevelIndex`))
    (`PlayerController.SetViewTargetWithBlend` _sokoban_player_controller (`self.TestCamera`) 0.0 "VTBlend_Linear" 0.0 false)
    (`/Game/Sokoban/Blueprint/Gameplay/BP_SokobanController.SwitchToGameplayInput` _sokoban_player_controller)
    (bind _returnvalue_7 (`|CreateWidget` "/Game/Sokoban/Blueprint/UI/WBP_HUD.WBP_HUD_C"))
    (`UserWidget.AddToViewport` _returnvalue_7 0)
    (else
      (`self.LoadLevelByIndex` 0))))

(fn `AddUndoState`
  (bind _undostate (`self.CurrentUndoState`))
  (`KismetArrayLibrary.Array_Add` (`self.UndoStack`) _undostate)
  ; 限制步数
  (if (> (`KismetArrayLibrary.Array_Length` (`self.UndoStack`)) (`self.MaxUndoSteps`))
    (`KismetArrayLibrary.Array_Remove` (`self.UndoStack`))))

(fn `CurrentUndoState`
  (returns (UndoState :type "/Game/Sokoban/Blueprint/Structure/ST_UndoState Structure"))
  (locals (L_BoxCoords :type "Array of /Game/Sokoban/Blueprint/Structure/ST_GridCoord Structure"))
  (bind _playerref (`self.PlayerRef`))
  (for _array_element (`self.SpawnedBoxes`)
    (`KismetArrayLibrary.Array_Add` (`local.L_BoxCoords`) (make `/Game/Sokoban/Blueprint/Structure/ST_GridCoord` (`/Game/Sokoban/Blueprint/Gameplay/BP_BoxActor.CurrentX` _array_element) (`/Game/Sokoban/Blueprint/Gameplay/BP_BoxActor.CurrentY` _array_element))))
  (return (make `/Game/Sokoban/Blueprint/Structure/ST_UndoState` (make `/Game/Sokoban/Blueprint/Structure/ST_GridCoord` (`/Game/Sokoban/Blueprint/Characters/BP_Player.CurrentX` _playerref) (`/Game/Sokoban/Blueprint/Characters/BP_Player.CurrentY` _playerref)) (`local.L_BoxCoords`))))

(fn `HandleLevelSuccess`
  (if (`self.TestLevelManager`)
    (`KismetSystemLibrary.PrintString` "Success")
    (else
      (`/Game/Sokoban/Blueprint/Gameplay/BP_FlowManager.ReturnToLevelSelectAfterSuccess` (`self.FlowManagerRef`) (`self.CurrentLevelIndex`)))))

(fn `LoadLevelByIndex`
  (params (LevelIndex :type Integer))
  (bind _successpanelref (`self.SuccessPanelRef`))
  (bind _spawnedboxes (`self.SpawnedBoxes`))
  (bind _playerref (`self.PlayerRef`))
  (bind _gridmanagerref (`self.GridManagerRef`))
  (bind _gridmanagerref_2 (`self.GridManagerRef`))
  (bind (_levelname _width _height _floorcells _wallcells _goalcells _boxcells _playerstart) (break `/Game/Sokoban/Blueprint/Structure/ST_LevelData` (`|GetArrayItem` (`self.LevelList`) (`local.LevelIndex`))))
  (bind (_x _y) (break `/Game/Sokoban/Blueprint/Structure/ST_GridCoord` _playerstart))
  (`|ExecutionSequence`
    (:`then_0`
      (set `self.CurrentLevelIndex` (`local.LevelIndex`))
      (`KismetArrayLibrary.Array_Clear` (`self.UndoStack`))
      (for _array_element _spawnedboxes
        (`self.K2_DestroyActor` _array_element))
      (`KismetArrayLibrary.Array_Clear` _spawnedboxes)
      ; 清空结算界面（如果有
      (`/Engine/EditorBlueprintResources/StandardMacros.IsValid` _successpanelref
        (:`Is Valid`
          (`Widget.SetVisibility` _successpanelref "Hidden"))))
    (:`then_1`
      ; Init
      (set `/Game/Sokoban/Blueprint/Gameplay/BP_GridManager.GridWidth` _width _gridmanagerref_2)
      (set `/Game/Sokoban/Blueprint/Gameplay/BP_GridManager.GridHeight` _height _gridmanagerref_2)
      (set `/Game/Sokoban/Blueprint/Gameplay/BP_GridManager.FloorCells` _floorcells _gridmanagerref_2)
      (set `/Game/Sokoban/Blueprint/Gameplay/BP_GridManager.WallCells` _wallcells _gridmanagerref_2)
      (set `/Game/Sokoban/Blueprint/Gameplay/BP_GridManager.GoalCells` _goalcells _gridmanagerref_2)
      (set `/Game/Sokoban/Blueprint/Gameplay/BP_GridManager.BoxCells` _boxcells _gridmanagerref_2)
      (set `/Game/Sokoban/Blueprint/Gameplay/BP_GridManager.PlayerPreview` _playerstart _gridmanagerref_2)
      (`/Game/Sokoban/Blueprint/Gameplay/BP_GridManager.BuildGridVisuals` _gridmanagerref_2 false)
      (set `/Game/Sokoban/Blueprint/Characters/BP_Player.CurrentX` _x _playerref)
      (set `/Game/Sokoban/Blueprint/Characters/BP_Player.CurrentY` _y _playerref)
      (`/Game/Sokoban/Blueprint/Characters/BP_Player.SnapToCurrentGrid` _playerref))
    (:`then_2`
      ; Spawn Boxes
      (for _array_element_2 (`/Game/Sokoban/Blueprint/Gameplay/BP_GridManager.BoxCells` (`self.GridManagerRef`))
        (bind (_x_2 _y_2) (break `/Game/Sokoban/Blueprint/Structure/ST_GridCoord` _array_element_2))
        (bind _returnvalue (`|SpawnActorFromClass` "/Game/Sokoban/Blueprint/Gameplay/BP_BoxActor.BP_BoxActor_C" (`KismetMathLibrary.MakeTransform` (0.0 0.0 -10.0) (struct) (1.8 1.8 1.8)) "Undefined" "MultiplyWithRoot" null _x_2 _y_2 null))
        (`/Game/Sokoban/Blueprint/Gameplay/BP_BoxActor.Init` _returnvalue)
        (`KismetArrayLibrary.Array_Add` (`self.SpawnedBoxes`) _returnvalue)
        (bind _worldlocation (`/Game/Sokoban/Blueprint/Gameplay/BP_GridManager.GridToWorld` _gridmanagerref _array_element_2))
        (`/Game/Sokoban/Blueprint/Gameplay/BP_GridManager.AddFloorInstrnce` _gridmanagerref _worldlocation)))
    (:`then_3`
      (if (`self.TestLevelManager`)
        (`/Game/Sokoban/Blueprint/Gameplay/BP_GridManager.CenterCamera` (`self.GridManagerRef`) (`self.TestCamera`))
        (else
          (`/Game/Sokoban/Blueprint/Gameplay/BP_GridManager.CenterCamera` (`self.GridManagerRef`) (`/Game/Sokoban/Blueprint/Gameplay/BP_FlowManager.GameplayCameraRef` (`self.FlowManagerRef`))))))))

(fn `LoadNextLevel`
  (`self.LoadLevelByIndex` (+ (`self.CurrentLevelIndex`) 1)))

(fn `RestartCurrentLevel`
  (`self.LoadLevelByIndex` (`self.CurrentLevelIndex`)))

(fn `RestoreUndoState`
  (params (InState :type "/Game/Sokoban/Blueprint/Structure/ST_UndoState Structure"))
  (bind _playerref (`self.PlayerRef`))
  (bind (_x _y) (break `/Game/Sokoban/Blueprint/Structure/ST_GridCoord` (`.PlayerCoord_3_8EAC92894DCFB6E5F171CCAAAE51AA65` (break `/Game/Sokoban/Blueprint/Structure/ST_UndoState` InState))))
  (set `/Game/Sokoban/Blueprint/Characters/BP_Player.CurrentX` _x _playerref)
  (set `/Game/Sokoban/Blueprint/Characters/BP_Player.CurrentY` _y _playerref)
  (`/Game/Sokoban/Blueprint/Characters/BP_Player.SnapToCurrentGrid` _playerref)
  (for (_array_element _array_index) (`self.SpawnedBoxes`)
    (bind (_output_x _output_y) (break `/Game/Sokoban/Blueprint/Structure/ST_GridCoord` (`|GetArrayItem` (`.BoxCoords_6_C2C22F1B4A414F48F3203FB43EE52483` (break `/Game/Sokoban/Blueprint/Structure/ST_UndoState` (`local.InState`))) _array_index)))
    (set `/Game/Sokoban/Blueprint/Gameplay/BP_BoxActor.CurrentX` _output_x _array_element)
    (set `/Game/Sokoban/Blueprint/Gameplay/BP_BoxActor.CurrentY` _output_y _array_element)
    (`/Game/Sokoban/Blueprint/Gameplay/BP_BoxActor.SnapToCurrentGrid` _array_element)
    (`/Game/Sokoban/Blueprint/Gameplay/BP_BoxActor.RefreshGoalState` _array_element)))

(fn `UndoLastStep`
  (locals (L_TargetState :type "/Game/Sokoban/Blueprint/Structure/ST_UndoState Structure"))
  (bind _returnvalue (`KismetArrayLibrary.Array_Length` (`self.UndoStack`)))
  (bind _returnvalue_2 (- _returnvalue 1))
  (if (not (== _returnvalue 0))
    (set `local.L_TargetState` (`|GetArrayItem` (`self.UndoStack`) _returnvalue_2))
    (`self.RestoreUndoState` (`local.L_TargetState`))
    (`KismetArrayLibrary.Array_Remove` (`self.UndoStack`) _returnvalue_2)))

(fn `UpdataLevelList`
  (params (LevelList :type "Array of /Game/Sokoban/Blueprint/Structure/ST_LevelData Structure"))
  (set `self.LevelList` LevelList))

(fn `UserConstructionScript`)