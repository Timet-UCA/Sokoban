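; Sokoban player actor that moves on a cell grid, pushes boxes and detects level completion.
; TryMove queries BP_GridManager for blocked cells and boxes, allowing a push only into a free cell.
; Valid moves record an undo state in BP_LevelManager, update the grid coordinates, then teleport-free snap the actor to its world position.
; Each snap checks whether boxes cover all goal cells and notifies the level manager on success.
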(event `self.ReceiveBeginPlay`
  (bind _returnvalue (`GameplayStatics.GetActorOfClass` "/Game/Sokoban/Blueprint/Gameplay/BP_GridManager.BP_GridManager_C"))
  (set `self.GridManagerRef` _returnvalue)
  (bind _returnvalue_2 (`GameplayStatics.GetActorOfClass` "/Game/Sokoban/Blueprint/Gameplay/BP_LevelManager.BP_LevelManager_C"))
  (set `self.LevelManagerRef` _returnvalue_2)
  (`self.SnapToCurrentGrid`))

(fn `CheckLevelSuccess`
  (locals (_UnSuccess :type Boolean))
  (`/Engine/EditorBlueprintResources/StandardMacros.IsValid` (`self.GridManagerRef`)
    (:`Is Valid`
      (if (not (== (`KismetArrayLibrary.Array_Length` (`/Game/Sokoban/Blueprint/Gameplay/BP_GridManager.GoalCells` (`self.GridManagerRef`))) 0))
        (bind _boxes (`/Game/Sokoban/Blueprint/Gameplay/BP_GridManager.GetAllBoxCoord` (`self.GridManagerRef`)))
        (for _array_element (`/Game/Sokoban/Blueprint/Gameplay/BP_GridManager.GoalCells` (`self.GridManagerRef`))
          (if (not (`KismetArrayLibrary.Array_Contains` _boxes _array_element))
            (set `local._UnSuccess` true)))
        (if (not (`local._UnSuccess`))
          (bind _returnvalue (`GameplayStatics.GetActorOfClass` "/Game/Sokoban/Blueprint/Gameplay/BP_LevelManager.BP_LevelManager_C"))
          (`/Game/Sokoban/Blueprint/Gameplay/BP_LevelManager.HandleLevelSuccess` _returnvalue))))))

(fn `SnapToCurrentGrid`
  (bind _gridmanagerref (`self.GridManagerRef`))
  (`/Engine/EditorBlueprintResources/StandardMacros.IsValid` _gridmanagerref
    (:`Is Valid`
      (bind _worldlocation (`/Game/Sokoban/Blueprint/Gameplay/BP_GridManager.GridToWorld` _gridmanagerref (make `/Game/Sokoban/Blueprint/Structure/ST_GridCoord` (`self.CurrentX`) (`self.CurrentY`))))
      (`self.K2_SetActorLocation` _worldlocation)
      (`self.CheckLevelSuccess`))))

(fn `TryMove`
  (params (DeltaX :type Integer) (DeltaY :type Integer))
  (locals (_TargetCoord :type "/Game/Sokoban/Blueprint/Structure/ST_GridCoord Structure") (_BoxTargetCoord :type "/Game/Sokoban/Blueprint/Structure/ST_GridCoord Structure") (_TargetBox :type "/Game/Sokoban/Blueprint/Gameplay/BP_BoxActor Object Reference"))
  (bind (__targetcoord_x __targetcoord_y) (break `/Game/Sokoban/Blueprint/Structure/ST_GridCoord` (`local._TargetCoord`)))
  (bind (__boxtargetcoord_x __boxtargetcoord_y) (break `/Game/Sokoban/Blueprint/Structure/ST_GridCoord` (`local._BoxTargetCoord`)))
  (bind (_x _y) (break `/Game/Sokoban/Blueprint/Structure/ST_GridCoord` (`local._TargetCoord`)))
  (bind (_x_2 _y_2) (break `/Game/Sokoban/Blueprint/Structure/ST_GridCoord` (`local._TargetCoord`)))
  (`/Engine/EditorBlueprintResources/StandardMacros.IsValid` (`self.GridManagerRef`)
    (:`Is Valid`
      (set `local._TargetCoord` (make `/Game/Sokoban/Blueprint/Structure/ST_GridCoord` (+ (`self.CurrentX`) (`local.DeltaX`)) (+ (`self.CurrentY`) (`local.DeltaY`))))
      (if (`/Game/Sokoban/Blueprint/Gameplay/BP_GridManager.CellBlocked` (`self.GridManagerRef`) (`local._TargetCoord`))
        (return)
        (else
          (bind _box (`/Game/Sokoban/Blueprint/Gameplay/BP_GridManager.GetCurrentBox` (`self.GridManagerRef`) (`local._TargetCoord`)))
          (`/Engine/EditorBlueprintResources/StandardMacros.IsValid` _box
            (:`Is Valid`
              (set `local._TargetBox` _box)
              (set `local._BoxTargetCoord` (make `/Game/Sokoban/Blueprint/Structure/ST_GridCoord` (+ __targetcoord_x (`local.DeltaX`)) (+ __targetcoord_y (`local.DeltaY`))))
              (if (not (or (`/Game/Sokoban/Blueprint/Gameplay/BP_GridManager.CellBlocked` (`self.GridManagerRef`) (`local._BoxTargetCoord`)) (`/Game/Sokoban/Blueprint/Gameplay/BP_GridManager.IsBox` (`self.GridManagerRef`) (`local._BoxTargetCoord`))))
                (`/Game/Sokoban/Blueprint/Gameplay/BP_LevelManager.AddUndoState` (`self.LevelManagerRef`))
                (`/Game/Sokoban/Blueprint/Gameplay/BP_BoxActor.MoveToCell` (`local._TargetBox`) __boxtargetcoord_x __boxtargetcoord_y)
                (set `self.CurrentX` _x_2)
                (set `self.CurrentY` _y_2)
                (`self.SnapToCurrentGrid`)))
            (:`Is Not Valid`
              (`/Game/Sokoban/Blueprint/Gameplay/BP_LevelManager.AddUndoState` (`self.LevelManagerRef`))
              (set `self.CurrentX` _x)
              (set `self.CurrentY` _y)
              (`self.SnapToCurrentGrid`))))))))

(fn `UserConstructionScript`)